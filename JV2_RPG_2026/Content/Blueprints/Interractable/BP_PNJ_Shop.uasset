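; BP_PNJ_Shop is an interactable shop NPC that opens and closes an in-world shop view for the player.
; Interact blends the camera to the NPC, shows its widget component, initializes WBP_Shop with itself, and flags the TopDownController as in-shop with movement disabled.
; ExitShop hides the widget, restores movement, clears the in-shop flag and blends the camera back to the controlled pawn.
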(event Custom|ExitShop
  (bind _playercontroller (CallFunction|GetTopDownController))
  (bind _playercontroller_2 (CallFunction|GetTopDownController))
  (Rendering|SetVisibility (Variables|Default|GetWidget) false false)
  (Variables|/Game/TopDown/Blueprints/BP_TopDownController.BP_TopDownController_C|SetShouldMove _playercontroller_2 true)
  (Game|Player|SetViewTargetwithBlend _playercontroller (Pawn|GetControlledPawn _playercontroller) 1.0 "VTBlend_Linear" 0.0 false)
  (Variables|/Game/TopDown/Blueprints/BP_TopDownController.BP_TopDownController_C|SetIsInShop _playercontroller_2 false)
  (Default|IsVisible _playercontroller_2))

(event EventInterract
  (bind _playercontroller (CallFunction|GetTopDownController))
  (bind _widget (Variables|Default|GetWidget))
  (Game|Player|SetViewTargetwithBlend (CallFunction|GetTopDownController) self 1.0 "VTBlend_Linear" 1.0 false)
  (Rendering|SetVisibility _widget true false)
  (bind _aswbp_shop (Utilities|Casting|CastToWBP_Shop (UserInterface|GetWidget _widget)))
  (Default|InitializeShop _aswbp_shop self)
  (Variables|/Game/TopDown/Blueprints/BP_TopDownController.BP_TopDownController_C|SetShouldMove _playercontroller false)
  (Variables|/Game/TopDown/Blueprints/BP_TopDownController.BP_TopDownController_C|SetIsInShop _playercontroller true)
  (Default|IsVisible _playercontroller))

(fn ConstructionScript
  (|CallParentFunction))