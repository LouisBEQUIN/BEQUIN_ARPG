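; BP_spawner_brosse is a spawner actor that creates a BP_Brosse whenever it is flagged as dead, likely to respawn it.
; UpdateIsdead sets the Isdead flag, and Tick polls it every frame, spawning the brosse slightly above the spawner's location and clearing the flag.
; Tick also prints the Isdead value to screen every frame as debug output.
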(event EventBeginPlay)

(event Collision|EventActorBeginOverlap
  (params (OtherActor :type Actor%20Object%20Reference)))

(event EventTick
  (params (DeltaSeconds :type Float%20%28single-precision%29))
  (Development|PrintString (Utilities|String|ToString(Boolean) (Variables|Default|GetIsdead)) true true "(R=0.000000,G=0.660000,B=1.000000,A=1.000000)" 0.0)
  (if (Variables|Default|GetIsdead)
    (Game|SpawnActorfromClass "/Game/Blueprints/BP_Brosse.BP_Brosse_C" (Math|Transform|MakeTransform (+ (Transformation|GetActorLocation self) "0.000000,0.000000,50.000000")) "Undefined" "MultiplyWithRoot" 0 0 0)
    (Variables|Default|SetIsdead false)))

(fn ConstructionScript)

(fn UpdateIsdead
  (Variables|Default|SetIsdead true))