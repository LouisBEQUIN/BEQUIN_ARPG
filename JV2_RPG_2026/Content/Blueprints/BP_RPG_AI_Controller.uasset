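; AI controller for an RPG enemy that runs the main behavior tree and keeps the enemy's HP.
; BeginPlay sets up the blackboard, stores the player pawn under the PlayerPosition key and starts the tree.
; LoseennemyHP subtracts a fixed amount of HP.
; Tick prints HP and destroys the controller itself, not the pawn, while HP is above zero, which looks inverted.
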(event EventBeginPlay
  (bind _blackboardcomponent (Class|AIController|UseBlackboard "/Game/AI/BB_MainBehaviourBlackBoard.BB_MainBehaviourBlackBoard"))
  (Variables|Default|SetBlackboard%20Component _blackboardcomponent)
  (AI|Components|Blackboard|SetValueasObject (Variables|Default|GetBlackboard%20Component) (Utilities|Name|MakeLiteralName "PlayerPosition") (Game|Player|GetPlayerPawn 0))
  (AI|RunBehaviorTree "/Game/AI/BT_MainBehaviour.BT_MainBehaviour"))

(event EventTick
  (params (DeltaSeconds :type Float%20%28single-precision%29))
  (Development|PrintString (Utilities|String|ToString(Integer) (Variables|Default|Getennemy_hp)) true true "(R=0.000000,G=0.660000,B=1.000000,A=1.000000)" 0.0)
  (if (not (<= (Variables|Default|Getennemy_hp) 0))
    (Actor|DestroyActor)))

(fn ConstructionScript)

(fn LoseennemyHP
  (Variables|Default|Setennemy_hp (- (Variables|Default|Getennemy_hp) 20)))